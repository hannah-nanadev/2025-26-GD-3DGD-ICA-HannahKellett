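; BP_InvComponent is an inventory component that holds an item array and manages its on-screen inventory widget.
; On BeginPlay it creates a WB_Inventory widget, sizes Items to a fixed slot count, and passes itself to the widget's LoadInventory.
; The IA_Inventory input action toggles the widget by adding it to or removing it from the viewport, based on its visibility.
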(event `self.ReceiveBeginPlay`
  (bind _returnvalue (`|CreateWidget` "/Game/_project/Inventory/Widgets/WB_Inventory.WB_Inventory_C"))
  (set `self.InventoryWidget` _returnvalue)
  (`KismetArrayLibrary.Array_Resize` (`self.Items`) 20)
  (`/Game/_project/Inventory/Widgets/WB_Inventory.LoadInventory` (`self.InventoryWidget`) self))

(event `EnhancedInput|/Game/_project/Input/Actions/IA_Inventory`
  (params (ActionValue :type Boolean) (ElapsedSeconds :type "Float (double-precision)") (TriggeredSeconds :type "Float (double-precision)") (InputAction :type "InputAction Object Reference" :default "/Game/_project/Input/Actions/IA_Inventory.IA_Inventory"))
  (bind _inventorywidget (`self.InventoryWidget`))
  (:`Triggered`
    (if (`Widget.IsVisible` _inventorywidget)
      (`Widget.RemoveFromParent` _inventorywidget)
      (else
        (`UserWidget.AddToViewport` _inventorywidget 0)))))