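; Dialogue_C holds a list of dialogue lines and feeds them to the player character one at a time when its Speaking event fires.
; If the player reports no message in progress, it passes the current line, text delay, waveform settings, frequency range and harmony multiplier to SpeakingMessage.
; It then advances the line index, wrapping to the first line after the last.
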(event `Speaking`
  (bind _returnvalue (`GameplayStatics.GetPlayerCharacter` 0))
  (bind _dialogue (`self.Dialogue`))
  (bind _bspeaking (message `/Game/_project/Blueprints/Player_BPI.CheckSpeaking` _returnvalue))
  (if (not _bspeaking)
    (message `/Game/_project/Blueprints/Player_BPI.Speaking` _returnvalue (`|GetArrayItem` _dialogue (`self.Current Dialogue`)) (`self.TextDelay`) (`self.Sine 1`) (`self.Sine 2`) (`self.Square 1`) (`self.Square 2`) (`self.Saw 1`) (`self.Saw 2`) (`self.Minimum Frequency`) (`self.Maximum Frequency`) (`self.Harmony Multiplier`))
    (bind _result (`/Engine/EditorBlueprintResources/StandardMacros.IncrementInt` (`self.Current Dialogue`))
      (:`  `
        (if (>= _result (`KismetArrayLibrary.Array_Length` _dialogue))
          (set `self.Current Dialogue` 0))))))