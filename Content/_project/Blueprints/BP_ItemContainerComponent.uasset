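; Item container component that gives the player a single item when its container is interacted with.
; It starts full on BeginPlay.
; On first interaction it shows pickup dialogue under the container's name, adds the item to the player's inventory and marks itself empty.
; Later interactions only show the empty dialogue.
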(event `self.ReceiveBeginPlay`
  (set `self.ContainsItem` true))

(event `Container Interacted`
  (params (Player :type "/Game/ThirdPerson/Blueprints/BP_ThirdPersonCharacter Object Reference"))
  (if (`self.ContainsItem`)
    (`/Game/ThirdPerson/Blueprints/BP_ThirdPersonCharacter.Speaking` Player (`self.PickupDialogue`) (`self.Container Name`) 0.0 true true false false false false 750.0 850.0 0.5)
    (`/Game/ThirdPerson/Blueprints/BP_ThirdPersonCharacter.AddItemToInventory` Player (`self.Item`))
    (set `self.ContainsItem` false)
    (else
      (`/Game/ThirdPerson/Blueprints/BP_ThirdPersonCharacter.Speaking` Player (`self.EmptyDialogue`) (`self.Container Name`) 0.0 true true false false false false 750.0 850.0 0.5))))