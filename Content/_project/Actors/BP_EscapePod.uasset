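; BP_EscapePod is an escape pod actor that stays hidden from BeginPlay until ActivatePod reveals it and enables its tick.
; Each tick advances a distance by Speed and moves the Sphere component to that point on the actor's Spline in local space.
; Fixed offsets adjust the sphere's height and yaw, and the Blueprint has no check for reaching the spline's end.
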(event `self.ReceiveBeginPlay`
  (`self.SetActorHiddenInGame` true))

(event `ActivatePod`
  (`self.SetActorHiddenInGame` false)
  (`self.SetActorTickEnabled` true))

(event `self.ReceiveTick`
  (params (DeltaSeconds :type "Float (single-precision)"))
  (bind _returnvalue (`SplineComponent.GetTransformAtDistanceAlongSpline` (`self.Spline`) (`self.DistanceAlongSpline`) "Local" false))
  (set `self.DistanceAlongSpline` (+ (* DeltaSeconds (`self.Speed`)) (`self.DistanceAlongSpline`)))
  (`SceneComponent.K2_SetRelativeTransform` (`self.Sphere`) (`KismetMathLibrary.MakeTransform` (`KismetMathLibrary.MakeVector` (.x (.location _returnvalue)) (.y (.location _returnvalue)) (+ (.z (.location _returnvalue)) -90.0)) (`KismetMathLibrary.MakeRotator` (.roll (.rotation _returnvalue)) (.pitch (.rotation _returnvalue)) (+ (.yaw (.rotation _returnvalue)) -90.0)) (`SceneComponent.RelativeScale3D` (`self.Sphere`))) false false))

(fn `UserConstructionScript`)