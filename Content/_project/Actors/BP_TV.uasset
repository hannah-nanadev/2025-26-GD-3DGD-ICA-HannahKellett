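; BP_TV is a TV actor that explodes and releases the item it contains.
; Its Explode event plays a placeholder sound, spawns a Niagara explosion and spawns a BP_Item carrying ContainedItem at a fixed world-space offset.
; It launches that item's mesh with a fixed velocity-change impulse, then destroys itself.
; Nothing in this graph calls Explode.
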(event `Explode`
  (bind _location (.location (`self.GetTransform`)))
  (bind _returnvalue (`KismetMathLibrary.MakeVector` (+ (.x _location) 50.0) (- (.y _location) 50.0) (.z _location)))
  (`GameplayStatics.PlaySoundAtLocation` "/Game/_project/Sounds/explosion_placeholder_findcredit.explosion_placeholder_findcredit" _location (struct) 1.0 1.0 0.0 null null null null)
  (`NiagaraFunctionLibrary.SpawnSystemAtLocation` "/Game/_project/NiagaraSystems/Explosion.Explosion" _returnvalue (struct :`Pitch` 90.0 :`Yaw` 45.0 :`Roll` -90.0) (2.0 2.0 2.0))
  (bind _returnvalue_2 (`|SpawnActorFromClass` "/Game/_project/Inventory/Blueprints/BP_Item.BP_Item_C" (`KismetMathLibrary.MakeTransform` _returnvalue (.rotation (`self.GetTransform`)) (.scale (`self.GetTransform`))) "Undefined" "MultiplyWithRoot" null (`self.ContainedItem`) null))
  (`PrimitiveComponent.AddImpulse` (`/Game/_project/Inventory/Blueprints/BP_Item.StaticMesh` _returnvalue_2) (500.0 -500.0 500.0) "None" true)
  (`self.K2_DestroyActor`))

(fn `UserConstructionScript`)