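; BP_Safe is a three-state puzzle safe that gives the player its contained item.
; Each state swaps in its own dialogue component, and the first two also set an item-use component from UseCases.
; AttachDevice reveals a cylinder, darkens the nearby light and starts beeping and a looping blink that runs until the state changes.
; AddWater stops the device, relights the nearby light in orange and adds the item to the inventory.
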(event `self.ReceiveBeginPlay`
  (`SceneComponent.SetVisibility` (`self.Cylinder`) false true)
  (`AudioComponent.Stop` (`self.DeviceBeeping`))
  (set `self.State` 0)
  (bind _returnvalue (`GameplayStatics.GetActorOfClass` "/Game/ThirdPerson/Blueprints/BP_ThirdPersonCharacter.BP_ThirdPersonCharacter_C"))
  (set `self.Player` _returnvalue)
  (bind _returnvalue_2 (`AddComponent|NODE_AddBP_DialogueComponent-0` :`Name` (`|GetArrayItem` (`self.Names`) (`self.State`)) :`Cutscene ID` (`self.Cutscene ID`) :`Dialogue` (`self.InitialDialogue`)))
  (set `self.CurrentDialogueComponent` _returnvalue_2)
  (`self.Set Use Case`))

(event `AttachDevice`
  (set `self.State` 1)
  (`KismetSystemLibrary.DelayUntilNextFrame`)
  (`LightComponent.SetIntensity` (`Light.LightComponent` (`self.Nearby Light`)) 0.0)
  (`SceneComponent.SetVisibility` (`self.Cylinder`) true true)
  (`self.DeviceLightActive`)
  (`AudioComponent.Play` (`self.DeviceBeeping`) 0.0)
  (`self.Set Use Case`)
  (`ActorComponent.K2_DestroyComponent` (`self.CurrentDialogueComponent`))
  (bind _returnvalue (`AddComponent|NODE_AddBP_DialogueComponent-1` :`Name` (`|GetArrayItem` (`self.Names`) (`self.State`)) :`Cutscene ID` (`self.Cutscene ID`) :`Dialogue` (`self.AfterDeviceDialogue`)))
  (set `self.CurrentDialogueComponent` _returnvalue))

(event `AddWater`
  (bind _lightcomponent (`Light.LightComponent` (`self.Nearby Light`)))
  (set `self.State` 2)
  (`LightComponent.SetIntensity` _lightcomponent 160.0)
  (`LightComponent.SetLightColor` _lightcomponent (struct :`R` 1.0 :`G` 0.459902 :`B` 0.095652 :`A` 1.0) true)
  (`LightComponent.SetIntensity` (`self.PointLight`) 0.0)
  (`AudioComponent.Stop` (`self.DeviceBeeping`))
  (`ActorComponent.K2_DestroyComponent` (`self.CurrentUsableComponent`))
  (`ActorComponent.K2_DestroyComponent` (`self.CurrentDialogueComponent`))
  (bind _returnvalue (`AddComponent|NODE_AddBP_DialogueComponent-2` :`Name` (`|GetArrayItem` (`self.Names`) (`self.State`)) :`Cutscene ID` (`self.Cutscene ID`) :`Dialogue` (`self.FinalDialogue`)))
  (set `self.CurrentDialogueComponent` _returnvalue)
  (`/Game/ThirdPerson/Blueprints/BP_ThirdPersonCharacter.AddItemToInventory` (`self.Player`) (`self.ContainedItem`)))

(event `DeviceLightActive`
  (if (== (`self.State`) 1) :!label _label
    (`LightComponent.SetIntensity` (`self.PointLight`) 0.0)
    (`KismetSystemLibrary.Delay` 0.1)
    (`LightComponent.SetIntensity` (`self.PointLight`) 1000.0)
    (`KismetSystemLibrary.Delay` 0.4)
    (goto _label)
    (else
      (`LightComponent.SetIntensity` (`self.PointLight`) 0.0))))

(fn `Set Use Case`
  (bind _currentusablecomponent (`self.CurrentUsableComponent`))
  (`/Engine/EditorBlueprintResources/StandardMacros.IsValid` _currentusablecomponent
    (:`Is Valid`
      (`ActorComponent.K2_DestroyComponent` _currentusablecomponent))
    (:`Is Not Valid`
      _))
  (bind _returnvalue (`AddComponent|NODE_AddBP_ItemUsableComponent-1` :`UseCases` (`|MakeArray` (`|GetArrayItem` (`self.UseCases`) (`self.State`)))))
  (set `self.CurrentUsableComponent` _returnvalue))

(fn `UserConstructionScript`)