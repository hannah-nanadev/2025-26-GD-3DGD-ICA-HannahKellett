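; Cutscene controller actor that plays level sequences from an indexed array of cutscene actors.
; RollCutscene starts the chosen sequence unless it is already rolling, optionally toggling the player character's inventory.
; CutsceneEndReached pauses the sequence and waits for InputRecieved, which then stops it and clears the rolling state.
; Input received while not waiting stops every sequence as a workaround against getting stuck in cutscenes.
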(event `self.ReceiveBeginPlay`
  (set `self.Cutscene Rolling` false)
  (bind _returnvalue (`GameplayStatics.GetActorOfClass` "/Game/ThirdPerson/Blueprints/BP_ThirdPersonCharacter.BP_ThirdPersonCharacter_C"))
  (set `self.Player` _returnvalue))

(event `RollCutscene`
  (params (Index :type Integer) (`Cutscene Toggles Inventory` :type Boolean))
  (if (not (and (== (`self.Current Cutscene`) Index) (`self.Cutscene Rolling`)))
    (bind _output_get (set `self.Current Cutscene` Index))
    (`KismetSystemLibrary.PrintString` (`KismetStringLibrary.Concat_StrStr` "Rolling cutscene ID " (`KismetStringLibrary.Conv_IntToString` _output_get)))
    (`MovieSceneSequencePlayer.Play` (`LevelSequenceActor.SequencePlayer` (`|GetArrayItem` (`self.CutsceneActors`) (`self.Current Cutscene`))))
    (set `self.Cutscene Rolling` true)
    (if `Cutscene Toggles Inventory`
      (`/Game/_project/Blueprints/BP_InvComponent.ToggleInventory` (`/Game/ThirdPerson/Blueprints/BP_ThirdPersonCharacter.BP_InvComponent` (`self.Player`))))))

(event `CutsceneEndReached`
  (`MovieSceneSequencePlayer.Pause` (`LevelSequenceActor.SequencePlayer` (`|GetArrayItem` (`self.CutsceneActors`) (`self.Current Cutscene`))))
  (set `self.waiting` true))

(event `InputRecieved`
  (if (`self.waiting`)
    (set `self.waiting` false)
    (`MovieSceneSequencePlayer.Stop` (`LevelSequenceActor.SequencePlayer` (`|GetArrayItem` (`self.CutsceneActors`) (`self.Current Cutscene`))))
    (set `self.Cutscene Rolling` false)
    (else
      (for _array_element (`self.CutsceneActors`)
        (`MovieSceneSequencePlayer.Stop` (`LevelSequenceActor.SequencePlayer` _array_element))))))

(fn `UserConstructionScript`)