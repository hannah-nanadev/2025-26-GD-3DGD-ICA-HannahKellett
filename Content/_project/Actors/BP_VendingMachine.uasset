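; BP_VendingMachine is an interactable vending machine that gives the player an item and swaps its dialogue once looted.
; On BeginPlay it finds the third-person character and adds a dialogue component with the unlooted lines.
; LootMachine adds the item to the player's inventory, sets Looted, then replaces that component with a new one holding the looted lines.
; The construction script applies the screen material to the Door mesh.
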(event `self.ReceiveBeginPlay`
  (bind _returnvalue (`GameplayStatics.GetActorOfClass` "/Game/ThirdPerson/Blueprints/BP_ThirdPersonCharacter.BP_ThirdPersonCharacter_C"))
  (set `self.Player` _returnvalue)
  (set `self.Looted` false)
  (bind _returnvalue_2 (`AddComponent|NODE_AddBP_DialogueComponent-0` :`Name` (`self.Name`) :`Dialogue` (`self.UnlootedDialogueArray`)))
  (set `self.CurrentDialogueComponent` _returnvalue_2))

(event `LootMachine`
  (`/Game/ThirdPerson/Blueprints/BP_ThirdPersonCharacter.AddItemToInventory` (`self.Player`) (`self.Item`))
  (set `self.Looted` true)
  (`ActorComponent.K2_DestroyComponent` (`self.CurrentDialogueComponent`))
  (bind _returnvalue (`AddComponent|NODE_AddBP_DialogueComponent-1` :`Name` (`self.Name`) :`Dialogue` (`self.LootedDialogueArray`)))
  (set `self.CurrentDialogueComponent` _returnvalue))

(fn `UserConstructionScript`
  (`PrimitiveComponent.SetMaterial` (`self.Door`) 0 (`self.ScreenMat`)))